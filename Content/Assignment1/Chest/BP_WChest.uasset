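; BP_WChest is a chest Blueprint that adds player-change feedback when the chest is opened.
; Its OpentheChest event runs the parent logic, then casts through the game mode to the WB_Keys widget and calls CallOnPlayerChange.
; It then plays a possession sound cue and spawns a particle emitter at the chest, both skipped if either cast fails.
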(event `self.OpenTheChest`
  (bind _returnvalue (`self.K2_GetActorLocation` self))
  (`parent.OpenTheChest`)
  (bind _asassignment_1_game_mode (cast `Assignment1_GameMode` (`GameplayStatics.GetGameMode`)))
  (bind _aswb_keys (cast `/Game/Assignment1/UI/WB_Keys` (`Assignment1_GameMode.Widget` _asassignment_1_game_mode)))
  (`/Game/Assignment1/UI/WB_Keys.OnPlayerChange` _aswb_keys)
  (`GameplayStatics.PlaySoundAtLocation` "/Engine/EditorSounds/GamePreview/PossessPlayer_Cue.PossessPlayer_Cue" _returnvalue (struct) 1.0 1.0 0.0 null null null)
  (`GameplayStatics.SpawnEmitterAtLocation` "/Engine/Tutorial/SubEditors/TutorialAssets/TutorialParticleSystem.TutorialParticleSystem" _returnvalue))

(fn `UserConstructionScript`
  (`parent.UserConstructionScript`))