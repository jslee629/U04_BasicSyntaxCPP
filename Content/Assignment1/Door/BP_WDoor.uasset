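; BP_WDoor is a door Blueprint that adds UI and audio feedback to the OpentheDoor behavior inherited from its parent.
; After running the parent logic with the overlapping actors, it gets the WB_Keys widget from Assignment1_GameMode and calls CallOnPlayerChange on it.
; It then plays EndSimulate_Cue at the door's location if IsOpen is false, so the sound is skipped whenever either cast fails.
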(event `self.OpenTheDoor`
  (params (OverlappedActor :type "Actor Object Reference") (OtherActor :type "Actor Object Reference"))
  (`parent.OpenTheDoor` OverlappedActor OtherActor)
  (bind _asassignment_1_game_mode (cast `Assignment1_GameMode` (`GameplayStatics.GetGameMode`)))
  (bind _aswb_keys (cast `/Game/Assignment1/UI/WB_Keys` (`Assignment1_GameMode.Widget` _asassignment_1_game_mode)))
  (`/Game/Assignment1/UI/WB_Keys.OnPlayerChange` _aswb_keys)
  (if (not (`self.IsOpen`))
    (`GameplayStatics.PlaySoundAtLocation` "/Engine/EditorSounds/GamePreview/EndSimulate_Cue.EndSimulate_Cue" (`self.K2_GetActorLocation` self) (struct) 1.0 1.0 0.0 null null null)))

(fn `UserConstructionScript`
  (`parent.UserConstructionScript`))